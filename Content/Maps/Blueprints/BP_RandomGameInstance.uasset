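; Game instance that manages the player profile save, front-end menus and LAN multiplayer sessions for multiple game types.
; It loads or creates the user save and treats a non-empty player name as valid, showing user settings instead of the main menu otherwise.
; Per-game-type map lookups drive travel: hosting opens a listen-server lobby or falls back to that game's menu map, while joining takes the first session found.
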(event `SaveUserInfo`
  (`GameplayStatics.SaveGameToSlot` (`self.UserInfoSaveGame`) (`self.UserInfoSlotName`))
  (`self.UserInfoValid`))

(event `CheckUserSave`
  ;[1 1 1] Check User Info save
  (bind _returnvalue (`GameplayStatics.DoesSaveGameExist` (`self.UserInfoSlotName`)))
  (if _returnvalue
    (bind _returnvalue_2 (`GameplayStatics.LoadGameFromSlot` (`self.UserInfoSlotName`)))
    (bind _asuser_player_save_game (cast `/Game/Blueprints/UserPlayerSaveGame` _returnvalue_2))
    (set `self.UserInfoSaveGame` _asuser_player_save_game)
    (`self.UserInfoValid`)
    (else
      (`/Engine/EditorBlueprintResources/StandardMacros.IsValid` (`self.UserInfoSaveGame`)
        (:`Is Not Valid`
          (bind _returnvalue_3 (`GameplayStatics.CreateSaveGameObject` "/Game/Blueprints/UserPlayerSaveGame.UserPlayerSaveGame_C"))
          (set `self.UserInfoSaveGame` _returnvalue_3)
          (set `self.IsUserInfoValid?` false))))))

(event `ShowMainMenu`
  (params (MenuWidgetClass :type "UserWidget Class Reference"))
  (bind _returnvalue (`GameplayStatics.GetPlayerController` 0))
  ;[1 1 1] Main Menu
  (if (`self.IsUserInfoValid?`)
    (bind _returnvalue_2 (`|CreateWidget` MenuWidgetClass (`GameplayStatics.GetPlayerController` 0)))
    (`UserWidget.AddToViewport` _returnvalue_2 0)
    (`WidgetBlueprintLibrary.SetInputMode_UIOnlyEx` _returnvalue (`self.MainMenuWB`))
    (set `PlayerController.bShowMouseCursor` true _returnvalue)
    (else
      (`self.ShowUserSettings`))))

(event `ShowUserSettings`
  ;[1 1 1] User Settings
  (bind _returnvalue (`|CreateWidget` "/Game/Maps/UI/WB_UserSettings.WB_UserSettings_C" (`GameplayStatics.GetPlayerController` 0)))
  (bind _output_get (set `self.UserSettingsWB` _returnvalue))
  (`UserWidget.AddToViewport` _output_get 0))

(event `ShowChooseGame`
  ;[1 1 1] User Settings
  (bind _returnvalue (`|CreateWidget` "/Game/Maps/UI/WB_ChooseGame.WB_ChooseGame_C" (`GameplayStatics.GetPlayerController` 0)))
  (bind _output_get (set `self.ChooseGameWB` _returnvalue))
  (`UserWidget.AddToViewport` _output_get 0))

(event `TravelToGame`
  (params (GameType :type "/Game/Maps/Blueprints/GameEnum Enum" :default "NewEnumerator0"))
  ;[1 1 1] Travel to Game
  (`GameplayStatics.OpenLevel` (`BlueprintMapLibrary.Map_Find` (`self.MainMenuMaps`) GameType)))

(event `HostGame`
  (params (GameType :type "/Game/Maps/Blueprints/GameEnum Enum" :default "NewEnumerator0"))
  ;[1 1 1] Host Game
  (`CreateSessionCallbackProxy.CreateSession` (`GameplayStatics.GetPlayerController` 0) (`self.MaxNumberOfPlayers`) true
    (:`OnSuccess`
      (`GameplayStatics.OpenLevel` (`BlueprintMapLibrary.Map_Find` (`self.LobbyMaps`) GameType) true "listen"))
    (:`OnFailure`
      (`self.TravelToGame` GameType))))

(event `JoinGame`
  (bind _returnvalue (`GameplayStatics.GetPlayerController` 0))
  ;[1 1 1] Join Game
  (bind _results (`FindSessionsCallbackProxy.FindSessions` _returnvalue 0 true)
    (:`OnSuccess`
      (`JoinSessionCallbackProxy.JoinSession` _returnvalue (`|GetArrayItem` _results)))))