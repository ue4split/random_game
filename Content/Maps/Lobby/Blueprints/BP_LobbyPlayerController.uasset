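; Player controller for the lobby map that sets up the local player's lobby interface.
; On BeginPlay, only for the local controller, it creates the main lobby UI widget with a reference to itself and adds it to the viewport.
; It then switches input to UI only, focused on that widget, and shows the mouse cursor.
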(event `self.ReceiveBeginPlay`
  (if (`self.IsLocalPlayerController`)
    (`|ExecutionSequence`
      (:`then_0`
        ;[1 1 1] Init Lobby UI
        (bind _returnvalue (`|CreateWidget` "/Game/Maps/Lobby/Widgets/BP_UILobbyMain.BP_UILobbyMain_C" self self))
        (bind _output_get (set `self.UILobbyMain` _returnvalue))
        (`UserWidget.AddToViewport` _output_get 0))
      (:`then_1`
        ;[1 1 1] Set input mode and mouse pointer
        (`WidgetBlueprintLibrary.SetInputMode_UIOnlyEx` self (`self.UILobbyMain`))
        (set `self.bShowMouseCursor` true)))))

(fn `UserConstructionScript`)