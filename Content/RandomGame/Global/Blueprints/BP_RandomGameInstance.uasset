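; Game instance for a multi-game project that handles menu flow, the user profile save, level travel and online sessions.
; It loads or creates the profile save, and ShowMainMenu opens user settings until a player name exists.
; Hosting and debug LAN joining open lobby maps looked up by game type.
; Network and travel errors print and destroy the session, while Init applies a NetworkVersionOverride for source engine builds.
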(event `SaveUserInfo`
  (`GameplayStatics.SaveGameToSlot` (`self.UserInfoSaveGame`) (`self.UserInfoSlotName`))
  (`self.UserInfoValid`))

(event `CheckUserSave`
  ;[1 1 1] Check User Info save
  (bind _returnvalue (`GameplayStatics.DoesSaveGameExist` (`self.UserInfoSlotName`)))
  (if _returnvalue
    (bind _returnvalue_2 (`GameplayStatics.LoadGameFromSlot` (`self.UserInfoSlotName`)))
    (bind _asuser_player_save_game (cast `/Game/RandomGame/Global/Blueprints/UserPlayerSaveGame` _returnvalue_2)
      (:`then`
        (set `self.UserInfoSaveGame` _asuser_player_save_game)
        (`self.UserInfoValid`))
      (:`CastFailed`
        (`KismetSystemLibrary.PrintString` "Filed to desirialize saved game")))
    (else
      (`/Engine/EditorBlueprintResources/StandardMacros.IsValid` (`self.UserInfoSaveGame`)
        (:`Is Not Valid`
          (bind _returnvalue_3 (`GameplayStatics.CreateSaveGameObject` "/Game/RandomGame/Global/Blueprints/UserPlayerSaveGame.UserPlayerSaveGame_C"))
          (set `self.UserInfoSaveGame` _returnvalue_3)
          (set `self.IsUserInfoValid?` false))))))

(event `ShowMainMenu`
  (params (MenuWidgetClass :type "UserWidget Class Reference") (OwningPlayer :type "PlayerController Object Reference"))
  ;[1 1 1] Main Menu
  (`WidgetBlueprintLibrary.SetInputMode_UIOnlyEx` OwningPlayer (`self.MainMenuWB`))
  (set `PlayerController.bShowMouseCursor` true OwningPlayer)
  (if (`self.IsUserInfoValid?`)
    (bind _returnvalue (`|CreateWidget` MenuWidgetClass OwningPlayer))
    (`UserWidget.AddToViewport` _returnvalue 0)
    (else
      (`self.ShowUserSettings` OwningPlayer))))

(event `ShowUserSettings`
  (params (OwningPlayer :type "PlayerController Object Reference"))
  ;[1 1 1] User Settings
  (bind _returnvalue (`|CreateWidget` "/Game/RandomGame/Global/UI/WB_UserSettings.WB_UserSettings_C" OwningPlayer))
  (bind _output_get (set `self.UserSettingsWB` _returnvalue))
  (`UserWidget.AddToViewport` _output_get 0))

(event `ShowChooseGame`
  (params (OwningPlayer :type "PlayerController Object Reference"))
  ;[1 1 1] User Settings
  (bind _returnvalue (`|CreateWidget` "/Game/RandomGame/Global/UI/WB_ChooseGame.WB_ChooseGame_C" OwningPlayer))
  (bind _output_get (set `self.ChooseGameWB` _returnvalue))
  (`UserWidget.AddToViewport` _output_get 0))

(event `TravelToGame`
  (params (GameType :type "/Game/RandomGame/Global/Blueprints/GameEnum Enum" :default "NewEnumerator0"))
  ;[1 1 1] Travel to Game
  (`GameplayStatics.OpenLevel` (`BlueprintMapLibrary.Map_Find` (`self.MainMenuMaps`) GameType)))

(event `ShowHostServerMenu`
  (params (OwningPlayer :type "PlayerController Object Reference") (GameType :type "/Game/RandomGame/Global/Blueprints/GameEnum Enum" :default "NewEnumerator0") (bUseLAN :type Boolean))
  ;[1 1 1] Show Host Server Menu
  (switch `/Game/RandomGame/Global/Blueprints/GameEnum` GameType
    (:`NewEnumerator0`
      (`KismetSystemLibrary.PrintString` "Error"))
    (:`NewEnumerator1`
      (bind _returnvalue (`|CreateWidget` "/Game/RandomGame/PerfectBlend/UI/WB_HostServerMenu.WB_HostServerMenu_C" OwningPlayer GameType bUseLAN))
      (`UserWidget.AddToViewport` _returnvalue 0))
    (:`NewEnumerator2`
      (bind _returnvalue_2 (`|CreateWidget` "/Game/RandomGame/Megalomania/UI/GameMenus/WB_HostServerMenu.WB_HostServerMenu_C" OwningPlayer GameType bUseLAN))
      (`UserWidget.AddToViewport` _returnvalue_2 0))))

(event `HostGame`
  (params (PlayerController :type "PlayerController Object Reference") (MaxNumberOfPlayers :type Integer) (bUseLAN :type Boolean) (GameType :type "/Game/RandomGame/Global/Blueprints/GameEnum Enum" :default "NewEnumerator0"))
  ;[1 1 1] Host Game
  (`CreateSessionCallbackProxy.CreateSession` PlayerController MaxNumberOfPlayers bUseLAN
    (:`OnSuccess`
      (`GameplayStatics.OpenLevel` (`BlueprintMapLibrary.Map_Find` (`self.LobbyMaps`) GameType) true "listen"))
    (:`OnFailure`
      (`self.TravelToGame` GameType))))

(event `DestroySessionCaller`
  (params (PlayerController :type "PlayerController Object Reference"))
  (`DestroySessionCallbackProxy.DestroySession` PlayerController))

(event `JoinGameDEBUG`
  (params (PlayerController :type "PlayerController Object Reference") (GameType :type "/Game/RandomGame/Global/Blueprints/GameEnum Enum" :default "NewEnumerator0"))
  ;[1 1 1] Join Game
  (bind _results (`FindSessionsCallbackProxy.FindSessions` PlayerController 1 true)
    (:`OnSuccess`
      (if (> (`KismetArrayLibrary.Array_Length` _results) 0)
        (`JoinSessionCallbackProxy.JoinSession` PlayerController (`|GetArrayItem` _results)
          (:`OnSuccess`
            (`GameplayStatics.OpenLevel` (`BlueprintMapLibrary.Map_Find` (`self.LobbyMaps`) GameType)))
          (:`OnFailure`
            (`KismetSystemLibrary.PrintString` "Join failed")))
        (else
          (`KismetSystemLibrary.PrintString` "Zero sessions"))))
    (:`OnFailure`
      (`KismetSystemLibrary.PrintString` "Find failed"))))

(event `self.HandleNetworkError`
  (params (FailureType :type "ENetworkFailure Enum" :default "NetDriverAlreadyExists") (bIsServer :type Boolean))
  (`KismetSystemLibrary.PrintString` (`|GetEnumeratorNameAsString` FailureType))
  (`DestroySessionCallbackProxy.DestroySession` (`GameplayStatics.GetPlayerController` 0)
    (:`then`
      (switch `ENetworkFailure` FailureType))))

(event `self.HandleTravelError`
  (params (FailureType :type "ETravelFailure Enum" :default "NoLevel"))
  (`KismetSystemLibrary.PrintString` (`|GetEnumeratorNameAsString` FailureType))
  (`DestroySessionCallbackProxy.DestroySession` (`GameplayStatics.GetPlayerController` 0)
    (:`then`
      (switch `ETravelFailure` FailureType))))

(event `self.ReceiveInit`
  ;[1 1 1] NetworkVersionOverride for source engine builds
  (`KismetSystemLibrary.ExecuteConsoleCommand` "NetworkVersionOverride 13144385" null)
  (`KismetSystemLibrary.PrintString` "NetworkVersionOverride"))