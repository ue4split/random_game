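; BP_ResourceSpawner is a server-side actor that scatters ResourceClass actors on the surfaces below its box volume.
; On BeginPlay, the authority spawns InitialCount resources and starts a looping timer that adds one every SpawnInterval, while remote copies destroy themselves.
; SpawnOne traces downward on Visibility from random points in the box and spawns at the hit location, adjusting for collisions but always spawning.
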(event `self.ReceiveBeginPlay`
  (`/Engine/EditorBlueprintResources/ActorMacros.Switch Has Authority`
    (:`Authority`
      (bind _returnvalue (`KismetSystemLibrary.K2_SetTimerDelegate` (delegate `SpawnResource`) (`self.SpawnInterval`) true))
      (set `self.Timer` _returnvalue)
      (for _ (range (+ (`self.InitialCount`) 1))
        (`self.SpawnOne`)))
    (:`Remote`
      (`self.K2_DestroyActor`))))

(event `SpawnResource`
  (`self.SpawnOne`))

(fn `SpawnOne`
  (bind (_origin _boxextent) (`KismetSystemLibrary.GetComponentBounds` (`self.Box`)))
  (bind _returnvalue (`KismetMathLibrary.RandomPointInBoundingBox` _origin _boxextent))
  (bind _outhit (`KismetSystemLibrary.LineTraceSingle` _returnvalue (+ _returnvalue (0.0 0.0 -100000.0)) "TraceTypeQuery1"))
  (`|SpawnActorFromClass` (`self.ResourceClass`) (`KismetMathLibrary.MakeTransform` (`.Location` (`GameplayStatics.BreakHitResult` _outhit))) "AdjustIfPossibleButAlwaysSpawn" "OverrideRootScale" null null))

(fn `UserConstructionScript`)