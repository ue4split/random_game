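; BP_TreeResource is a harvestable tree resource actor that yields an amount to a player's task and falls over when depleted.
; Harvest subtracts from Amount and returns the harvested value with a depletion flag, calling work completion on the Task when empty.
; Depletion runs a timeline that rolls the static mesh, then destroys the actor on authority only.
; BeginPlay creates a dynamic material and initializes its fade parameter.
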(event `self.ReceiveBeginPlay`
  (bind _returnvalue (`PrimitiveComponent.CreateDynamicMaterialInstance` (`self.StaticMesh`) 0 null "None"))
  (bind _output_get (set `self.MID` _returnvalue))
  (`MaterialInstanceDynamic.SetScalarParameterValue` _output_get "FadeParam" 1.0))

(event `DestroyResource`
  (bind (_direction _animparam) (`Timeline|Timeline_disappear`)
    (:`Update`
      (`SceneComponent.K2_SetRelativeRotation` (`self.StaticMesh`) (`KismetMathLibrary.MakeRotator` _animparam) false false))
    (:`Finished`
      (`/Engine/EditorBlueprintResources/ActorMacros.Switch Has Authority`
        (:`Authority`
          (`self.K2_DestroyActor`))))))

(fn `GetCurrentAmount`
  (returns (Amount :type "Float (double-precision)"))
  (return (`self.Amount`)))

(fn `Harvest`
  (params (Amount :type "Float (double-precision)") (Player :type "/Game/RandomGame/Megalomania/BP_MegalomaniaPC Object Reference") (Task :type "/Game/RandomGame/Megalomania/Tasks/BP_TaskBase Object Reference"))
  (returns (Output :type "Float (double-precision)") (bIsDepleted :type Boolean))
  (locals (HarvestedAmount :type "Float (double-precision)" :default 0.0) (`bIsDepleted?` :type Boolean :default false))
  (set `local.HarvestedAmount` (`KismetMathLibrary.FMin` Amount (`self.Amount`)))
  (set `self.Amount` (- (`self.Amount`) (`local.HarvestedAmount`)))
  (set `local.bIsDepleted?` (== (`self.Amount`) 0.0))
  (if (`local.bIsDepleted?`)
    (`self.DestroyResource`)
    (`/Game/RandomGame/Megalomania/Tasks/BP_TaskBase.OnWorkComplete` (`local.Task`))
    (return (`local.HarvestedAmount`) (`local.bIsDepleted?`))
    (else
      (return (`local.HarvestedAmount`) (`local.bIsDepleted?`)))))

(fn `UserConstructionScript`)