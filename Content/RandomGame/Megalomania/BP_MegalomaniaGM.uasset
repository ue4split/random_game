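; BP_MegalomaniaGM is the game mode for the Megalomania game.
; It overrides SpawnDefaultPawnFor to spawn the default pawn class at the start spot's transform; a Possess call in that function is left unconnected.
; Restart player, post login and logout events only print debug strings.
; The SpawnBuildSite event in the GamePlay graph is an empty stub.
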(event `self.K2_OnRestartPlayer`
  (params (NewPlayer :type "Controller Object Reference"))
  (`KismetSystemLibrary.PrintString` "Restart Player"))

(event `self.K2_PostLogin`
  (params (NewPlayer :type "PlayerController Object Reference"))
  (`KismetSystemLibrary.PrintString` "Post Login"))

(event `self.K2_OnLogout`
  (params (ExitingController :type "Controller Object Reference"))
  (`KismetSystemLibrary.PrintString` "On Logout"))

(event `SpawnBuildSite`)

(fn `SpawnDefaultPawnFor`
  (params (NewPlayer :type "Controller Object Reference") (StartSpot :type "Actor Object Reference"))
  (returns (ReturnValue :type "Pawn Object Reference"))
  (bind _returnvalue (`|SpawnActorFromClass` (`self.DefaultPawnClass`) (`self.GetTransform` StartSpot) "Undefined" "OverrideRootScale" null null))
  (return _returnvalue))

(fn `UserConstructionScript`)