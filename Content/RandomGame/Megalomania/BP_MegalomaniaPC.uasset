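; Player controller for Megalomania that drives a view camera pawn, tree harvesting and building placement.
; Axis input pans and zooms the camera, while held click or touch moves it toward the hit point.
; An interaction state switches StartTask between adding harvest workers or tasks on trees and spawning build sites at a validated ghost's location.
; Ghost classes, build sites and costs come from a DataTable cached on BeginPlay.
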(event `InputAxis|ViewForward`
  (params (AxisValue :type "Float (single-precision)"))
  (bind _asbp_view_camera_character (cast `/Game/RandomGame/Megalomania/BP_ViewCameraCharacter` (`self.K2_GetPawn`)))
  (`/Game/RandomGame/Megalomania/BP_ViewCameraCharacter.MoveViewportDelta` _asbp_view_camera_character (`KismetMathLibrary.MakeVector` (* AxisValue (`self.ViewportMovementSensitivity`)))))

(event `self.ReceiveTick`
  (params (DeltaSeconds :type "Float (single-precision)"))
  (bind (_bblockinghit _binitialoverlap _time _distance _location _impactpoint _normal _impactnormal _physmat _hitactor) (`GameplayStatics.BreakHitResult` (`self.GetHitResultUnderCursorByChannel` "TraceTypeQuery1")))
  ;[1 1 1] Click and go there
  (`|ExecutionSequence`
    (:`then_0`
      (`/Engine/EditorBlueprintResources/StandardMacros.Gate` true :!label _label ; While key is pressed...
        (:`Exit`
          (`/Game/RandomGame/Megalomania/BP_ViewCameraCharacter.MoveViewportToHit` (cast `/Game/RandomGame/Megalomania/BP_ViewCameraCharacter` (`self.K2_GetPawn`) :!pure true) (`self.GetHitResultUnderCursorByChannel` "TraceTypeQuery1")))))
    (:`then_1`
      (`/Engine/EditorBlueprintResources/StandardMacros.Gate` true :!label _label_2 ; While finger is touching...
        (:`Exit`
          (`/Game/RandomGame/Megalomania/BP_ViewCameraCharacter.MoveViewportToHit` (cast `/Game/RandomGame/Megalomania/BP_ViewCameraCharacter` (`self.K2_GetPawn`) :!pure true) (`self.GetHitResultUnderFingerByChannel` (stale `InputTouch` FingerIndex) "TraceTypeQuery1")))))
    (:`then_2`
      (switch `/Game/RandomGame/Megalomania/DataTypes/InteractionState` (`self.Interaction State`)
        (:`NewEnumerator0`
          (bind _ghost_actor (`self.Ghost Actor`)
            (:`then`
              (`self.K2_DestroyActor` _ghost_actor))
            (:`else`)))
        (:`NewEnumerator1`
          (bind _ghost_actor_2 (`self.Ghost Actor`)
            (:`then`
              (`self.K2_SetActorLocation` _ghost_actor_2 _location false false))
            (:`else`
              (bind _returnvalue (`|SpawnActorFromClass` (`.BuildingGhost_12_0A8D48E96E7B4883B84D21F836F83E3C` (break `/Game/RandomGame/Megalomania/DataTypes/BuildingConfigStruct` (`BlueprintMapLibrary.Map_Find` (`self.BuildingConfig`) (`self.Building Class`)))) (`KismetMathLibrary.MakeTransform` _location) "Undefined" "OverrideRootScale" null null))
              (set `self.Ghost Actor` _returnvalue)))
          (`/Game/RandomGame/Megalomania/Tasks/Placement/BP_BuildingGhost.SetIsOnLandscape` (`self.Ghost Actor`) (`.bSuccess` (cast `Landscape` _hitactor :!pure true))))))))

(event `InputAction|SetDestination`
  (params (Key :type "Key Structure"))
  ;[1 1 1] Click and go there
  (:`Pressed`
    (goto _label :!via `Open`))
  (:`Released`
    (goto _label :!via `Close`)))

(event `InputAxis|ViewRight`
  (params (AxisValue :type "Float (single-precision)"))
  (bind _asbp_view_camera_character (cast `/Game/RandomGame/Megalomania/BP_ViewCameraCharacter` (`self.K2_GetPawn`)))
  (`/Game/RandomGame/Megalomania/BP_ViewCameraCharacter.MoveViewportDelta` _asbp_view_camera_character (`KismetMathLibrary.MakeVector` 0.0 (* AxisValue (`self.ViewportMovementSensitivity`)))))

(event `InputTouch`
  (params (Location :type "Vector Structure") (FingerIndex :type "ETouchIndex Enum"))
  (bind _returnvalue (`|EnumEquality` FingerIndex "Touch1"))
  ;[1 1 1] Click and go there
  (:`Pressed`
    (if _returnvalue
      (goto _label_2 :!via `Open`)))
  (:`Released`
    (if _returnvalue
      (goto _label_2 :!via `Close`))))

(event `InputAxis|ViewZoomIn`
  (params (AxisValue :type "Float (single-precision)"))
  (bind _asbp_view_camera_character (cast `/Game/RandomGame/Megalomania/BP_ViewCameraCharacter` (`self.K2_GetPawn`)))
  (`/Game/RandomGame/Megalomania/BP_ViewCameraCharacter.ZoomViewportDelta` _asbp_view_camera_character (* AxisValue (`self.ViewportZoomSensitivity`))))

(event `InputAction|StartTask`
  (params (Key :type "Key Structure"))
  (:`Pressed`
    (switch `/Game/RandomGame/Megalomania/DataTypes/InteractionState` (`self.Interaction State`)
      (:`NewEnumerator0`
        (bind _asbp_tree_resource (cast `/Game/RandomGame/Megalomania/Actors/BP_TreeResource` (`.HitActor` (`GameplayStatics.BreakHitResult` (`self.GetHitResultUnderCursorByChannel` "TraceTypeQuery1")))))
        (`self.AddHarvesterOrSpawnTask` _asbp_tree_resource))
      (:`NewEnumerator1`
        (if (`/Game/RandomGame/Megalomania/Tasks/Placement/BP_BuildingGhost.GetIsValidLocation` (`self.Ghost Actor`))
          (`self.SpawnBuildSite` (`.Location` (`GameplayStatics.BreakHitResult` (`self.GetHitResultUnderCursorByChannel` "TraceTypeQuery1"))) (`self.Building Class`))
          (set `self.Interaction State` "NewEnumerator0"))))))

(event `StartPlacingBuilding`
  (params (`Building Class` :type "/Game/RandomGame/Megalomania/Actors/BP_Building Class Reference"))
  (switch `/Game/RandomGame/Megalomania/DataTypes/InteractionState` (`self.Interaction State`)
    (:`NewEnumerator0`
      (set `self.Building Class` `Building Class`)
      (set `self.Interaction State` "NewEnumerator1"))
    (:`NewEnumerator1`
      (set `self.Interaction State` "NewEnumerator0"))))

(event `self.ReceiveBeginPlay`
  (`self.ReadConfig`))

(event `AddWorker`
  (params (Task :type "/Game/RandomGame/Megalomania/Tasks/BP_TaskBase Object Reference"))
  (`/Game/RandomGame/Megalomania/Tasks/BP_TaskBase.ChangeWorkers` Task 1))

(event `SpawnTask`
  (params (Resource :type "Actor Object Reference"))
  (bind _returnvalue (`|SpawnActorFromClass` "/Game/RandomGame/Megalomania/Tasks/Harvesting/BP_HarvestTreeTask.BP_HarvestTreeTask_C" (`KismetMathLibrary.MakeTransform` (0.0 0.0 0.0)) "Undefined" "OverrideRootScale" self 1 5.0 null))
  (`/Engine/EditorBlueprintResources/StandardMacros.IsValid` _returnvalue
    (:`Is Valid`
      (`/Game/RandomGame/Megalomania/Tasks/Harvesting/BP_HarvestTreeTask.AttachToResource` _returnvalue Resource))))

(event `SpawnBuildSite`
  (params (`Spawn Transform Location` :type "Vector Structure") (BuildingClass :type "/Game/RandomGame/Megalomania/Actors/BP_Building Class Reference (by ref)"))
  (bind ((`BuildSite_18_60E87B14D21240D3BE2C406252E52C92` _buildsite) (`ResourceCost_22_4116684261544D839F5162914D8E1B5E` _resourcecost) (`WorkAmount_24_79D5D09847C44837B0D84B1CDDFBF8AA` _workamount)) (break `/Game/RandomGame/Megalomania/DataTypes/BuildingConfigStruct` (`BlueprintMapLibrary.Map_Find` (`self.BuildingConfig`) BuildingClass)))
  (`|SpawnActorFromClass` _buildsite (`KismetMathLibrary.MakeTransform` `Spawn Transform Location`) "Undefined" "OverrideRootScale" self _resourcecost _workamount BuildingClass 1 5.0 null))

(fn `AddHarvesterOrSpawnTask`
  (params (Resource :type "Actor Object Reference"))
  (for _array_element (`self.GetAttachedActors` Resource true)
    (bind _asbp_harvest_tree_task (cast `/Game/RandomGame/Megalomania/Tasks/Harvesting/BP_HarvestTreeTask` _array_element))
    (`self.AddWorker` _asbp_harvest_tree_task)
    (return))
  (`self.SpawnTask` (`local.Resource`)))

(fn `ReadConfig`
  (bind _outrownames (`DataTableFunctionLibrary.GetDataTableRowNames` "/Game/RandomGame/Megalomania/Config/BuildingsConfigDataTable.BuildingsConfigDataTable"))
  (for _array_element _outrownames
    (bind _returnvalue (`|GetDataTableRow` "/Game/RandomGame/Megalomania/Config/BuildingsConfigDataTable.BuildingsConfigDataTable" _array_element)
      (:`then`
        (`BlueprintMapLibrary.Map_Add` (`self.BuildingConfig`) (`.BuildingType_9_9EDBF2C8A48043D4ABDA347F6131F1FE` (break `/Game/RandomGame/Megalomania/DataTypes/BuildingConfigStruct` _returnvalue)) _returnvalue)))))

(fn `UserConstructionScript`)