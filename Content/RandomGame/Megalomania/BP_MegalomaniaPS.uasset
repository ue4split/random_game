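; Player state for the Megalomania game, holding each player's color, population, available workers and resources.
; On BeginPlay the authority picks a random color from a fixed palette of six.
; Population and resource updates clamp at zero, and population changes recompute available workers by subtracting workers on task actors sharing the same owner.
; RepNotifies on available workers and resources broadcast change events.
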(event `self.ReceiveBeginPlay`
  (`/Engine/EditorBlueprintResources/ActorMacros.Switch Has Authority`
    (:`Authority`
      (set `self.PlayerColor` (`KismetArrayLibrary.Array_Random` (`|MakeArray` (struct :`R` 1.0 :`B` 0.62746 :`A` 1.0) (struct :`R` 1.0 :`G` 0.333052 :`A` 1.0) (struct :`G` 0.029788 :`B` 1.0 :`A` 1.0) (struct :`G` 0.609375 :`B` 0.131064 :`A` 1.0) (struct :`R` 0.866678 :`G` 1.0 :`A` 1.0) (struct :`R` 0.244792 :`G` 0.244792 :`B` 0.244792 :`A` 1.0) :!type "LinearColor Structure"))))))

(fn `OnRep_AvailableWorkers`
  (`self.OnPopulationChanged`))

(fn `OnRep_Resources`
  (`self.OnResourcesChanged`))

(fn `UpdateAvailable`
  (locals (Working :type Integer))
  (bind _outactors (`GameplayStatics.GetAllActorsOfClass` "/Game/RandomGame/Megalomania/Tasks/BP_TaskBase.BP_TaskBase_C"))
  (for _array_element _outactors
    (if (== (`self.GetOwner` _array_element) (`self.GetOwner`))
      (set `local.Working` (+ (`/Game/RandomGame/Megalomania/Tasks/BP_TaskBase.Workers` _array_element) (`local.Working`)))))
  (set `self.AvailableWorkers` (- (`self.Population`) (`local.Working`))))

(fn `UpdatePopulation`
  (params (PopulationChange :type Integer))
  (set `self.Population` (`KismetMathLibrary.Max` (+ PopulationChange (`self.Population`))))
  (`self.UpdateAvailable`))

(fn `UpdateResources`
  (params (ResourceChange :type "Float (double-precision)"))
  (set `self.Resources` (`KismetMathLibrary.FMax` (+ ResourceChange (`self.Resources`)))))

(fn `UserConstructionScript`
  (`self.UpdateAvailable`))