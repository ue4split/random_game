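; BP_ViewCameraCharacter is a possessable camera rig that provides viewport panning and zoom in Megalomania.
; It moves either to a hit location's X and Y at its starting height, or by a local-space delta without sweeping.
; Zoom accumulates into a clamped alpha that lerps spring arm length and pitch together between default and close-up views.
; Possession prints a debug message naming the pawn and controller.
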(event `self.ReceiveBeginPlay`
  (set `self.InitialLocation` (`self.K2_GetActorLocation`)))

(event `MoveViewportToHit`
  (params (Hit :type "HitResult Structure"))
  (bind (_initiallocation_x _initiallocation_y _initiallocation_z) (`KismetMathLibrary.BreakVector` (`self.InitialLocation`)))
  (`self.K2_SetActorLocation` (`KismetMathLibrary.MakeVector` (.x (`.Location` (`GameplayStatics.BreakHitResult` Hit))) (.y (`.Location` (`GameplayStatics.BreakHitResult` Hit))) _initiallocation_z)))

(event `MoveViewportDelta`
  (params (DeltaLocation :type "Vector Structure"))
  (`self.K2_AddActorLocalOffset` DeltaLocation))

(event `ZoomViewportDelta`
  (params (`Zoom Delta` :type "Float (double-precision)"))
  (bind _springarm (`self.SpringArm`))
  (bind _viewzoomcurrent (`self.ViewZoomCurrent`))
  (set `self.ViewZoomCurrent` (`KismetMathLibrary.FClamp` (+ `Zoom Delta` (`self.ViewZoomCurrent`))))
  (set `SpringArmComponent.TargetArmLength` (`KismetMathLibrary.Lerp` (`self.ViewDefaultArmLenght`) (`self.ViewCloseupArmLenght`) _viewzoomcurrent) _springarm)
  (`SceneComponent.K2_SetRelativeRotation` _springarm (`KismetMathLibrary.MakeRotator` 0.0 (`KismetMathLibrary.Lerp` (`self.ViewDefaultAngle`) (`self.ViewCloseupAngle`) _viewzoomcurrent)) false false))

(event `self.ReceivePossessed`
  (params (NewController :type "Controller Object Reference"))
  (`KismetSystemLibrary.PrintString` (`KismetTextLibrary.Conv_TextToString` (`|FormatText` "{pawn} possesed by {controller}" (`KismetSystemLibrary.GetDisplayName` null) (`KismetSystemLibrary.GetDisplayName` NewController)))))

(fn `UserConstructionScript`)