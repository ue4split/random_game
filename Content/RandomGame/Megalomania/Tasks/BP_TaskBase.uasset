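; Base task Blueprint for Megalomania that spends a player's workers on timed chunks of work.
; On authority it gets the owning controller's PlayerState, clamps Workers to those available, and frees them on destruction.
; Worker changes refresh availability and restart a looping timer whose period is ChunkInterval divided by Workers.
; Each tick fires OnChunkDone; OnWorkComplete has a broadcast event that nothing here triggers.
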(event `self.ReceiveBeginPlay`
  (`|ExecutionSequence`
    (:`then_0`
      (`/Engine/EditorBlueprintResources/ActorMacros.Switch Has Authority`
        (:`Authority`
          (set `self.PlayerState` (cast `/Game/RandomGame/Megalomania/BP_MegalomaniaPS` (`Controller.PlayerState` (cast `/Game/RandomGame/Megalomania/BP_MegalomaniaPC` (`self.GetOwner`) :!pure true)) :!pure true)))))
    (:`then_1`
      (`/Engine/EditorBlueprintResources/ActorMacros.Switch Has Authority`
        (:`Authority`
          (set `self.Workers` (`KismetMathLibrary.Clamp` (`self.Workers`) 0 (`/Game/RandomGame/Megalomania/BP_MegalomaniaPS.AvailableWorkers` (`self.PlayerState`))))
          (`/Game/RandomGame/Megalomania/BP_MegalomaniaPS.UpdateAvailable` (`self.PlayerState`)))))
    (:`then_2`
      (`self.SetupTimer`))))

(event `SetupTimer`
  (`/Engine/EditorBlueprintResources/ActorMacros.Switch Has Authority`
    (:`Authority`
      (`KismetSystemLibrary.K2_ClearAndInvalidateTimerHandle` (`self.Timer`))
      (if (!= (`self.Workers`) 0)
        (bind _returnvalue (`KismetSystemLibrary.K2_SetTimerDelegate` (delegate `ChunkEvent`) (/ (`self.ChunkInterval`) (`KismetMathLibrary.Conv_IntToDouble` (`self.Workers`))) true))
        (set `self.Timer` _returnvalue)))))

(event `ChunkEvent`
  (`self.BroadcastChunkDone`))

(event `BroadcastChunkDone`
  (`self.OnChunkDone`))

(event `BroadcastWorkComplete`
  (`self.OnWorkComplete`))

(event `self.ReceiveDestroyed`
  (`/Engine/EditorBlueprintResources/ActorMacros.Switch Has Authority`
    (:`Authority`
      (set `self.Workers` 0)
      (`/Game/RandomGame/Megalomania/BP_MegalomaniaPS.UpdateAvailable` (`self.PlayerState`)))))

(event `ChangeWorkers`
  (params (NumderOfWorkers :type Integer :default 7))
  (set `self.Workers` (`KismetMathLibrary.Max` (+ (`KismetMathLibrary.Min` NumderOfWorkers (`/Game/RandomGame/Megalomania/BP_MegalomaniaPS.AvailableWorkers` (`self.PlayerState`))) (`self.Workers`))))
  (`/Game/RandomGame/Megalomania/BP_MegalomaniaPS.UpdateAvailable` (`self.PlayerState`))
  (`self.SetupTimer`))

(fn `AddWorkers`
  (`self.ChangeWorkers` 7))

(fn `RemoveWorkers`
  (`self.ChangeWorkers` -7))

(fn `UserConstructionScript`)