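; BP_BuildSite is a construction-site task in Megalomania that turns paid-for work chunks into a finished building.
; Each completed chunk updates a material fade from the progress ratio, while the authority deducts that chunk's share of the cost and advances work only if affordable.
; At full progress it broadcasts completion, spawns the building owned by the PlayerState and destroys itself.
; An info widget is created only for the owning local player controller.
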(event `self.ReceiveBeginPlay`
  (`parent.ReceiveBeginPlay`)
  (`|ExecutionSequence`
    (:`then_0`
      (bind _returnvalue (`PrimitiveComponent.CreateDynamicMaterialInstance` (`self.StaticMesh`) 0 null "None"))
      (set `self.MID` _returnvalue)
      (`MaterialInstanceDynamic.SetScalarParameterValue` (`self.MID`) "FadeParam" 0.0)
      (`self.InitInfoWidget`))
    (:`then_1`
      (add `self.OnChunkDone` (delegate `OnChunkDone_Event1`)))))

(event `OnChunkDone_Event1`
  (`MaterialInstanceDynamic.SetScalarParameterValue` (`self.MID`) "FadeParam" (/ (`KismetMathLibrary.Conv_IntToDouble` (`self.WorkDone`)) (`KismetMathLibrary.Conv_IntToDouble` (`self.WorkAmount`))))
  (`/Engine/EditorBlueprintResources/ActorMacros.Switch Has Authority`
    (:`Authority`
      (bind _bisworkdone (`self.SpendResources`))
      (if _bisworkdone
        (`/Engine/EditorBlueprintResources/StandardMacros.IncrementInt` (`self.WorkDone`)
          (:`  `
            (if (>= (`self.WorkDone`) (`self.WorkAmount`))
              (`self.BroadcastWorkComplete`)
              (`|SpawnActorFromClass` (`self.BuildingClass`) (`self.GetTransform`) "AlwaysSpawn" "OverrideRootScale" (`self.PlayerState`) null)
              (`self.K2_DestroyActor`))))))))

(fn `InitInfoWidget`
  (bind _asbp_megalomania_pc (cast `/Game/RandomGame/Megalomania/BP_MegalomaniaPC` (`self.GetOwner`)))
  (if (`Controller.IsLocalPlayerController` _asbp_megalomania_pc)
    (bind _returnvalue (`|CreateWidget` "/Game/RandomGame/Megalomania/UI/InGame/WB_BuildTaskInfo.WB_BuildTaskInfo_C" _asbp_megalomania_pc self))
    (`WidgetComponent.SetWidget` (`self.TaskInfoWidget`) _returnvalue)))

(fn `SpendResources`
  (returns (bIsWorkDone :type Boolean))
  (locals (ChunkCost :type "Float (double-precision)" :default 0.0))
  (set `local.ChunkCost` (/ (`self.ResourceCost`) (`KismetMathLibrary.Conv_IntToDouble` (`self.WorkAmount`))))
  (if (>= (`/Game/RandomGame/Megalomania/BP_MegalomaniaPS.Resources` (`self.PlayerState`)) (`local.ChunkCost`))
    (`/Game/RandomGame/Megalomania/BP_MegalomaniaPS.UpdateResources` (`self.PlayerState`) (* (`local.ChunkCost`) -1.0))
    (return true)
    (else
      (return false))))

(fn `UserConstructionScript`
  (`parent.UserConstructionScript`))