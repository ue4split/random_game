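; BP_SmallHouseBuildSite is a small house construction site that shows build progress through its material.
; On BeginPlay it creates a dynamic material instance on StaticMesh0, starts FadeParam at zero and binds to the inherited OnChunkDone event.
; Each completed work chunk sets FadeParam to the ratio of WorkDone to WorkAmount, so the material tracks completion.
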(event `self.ReceiveBeginPlay`
  (`parent.ReceiveBeginPlay`)
  (add `self.OnChunkDone` (delegate `OnChunkDone_Event2`))
  (bind _returnvalue (`PrimitiveComponent.CreateDynamicMaterialInstance` (`self.StaticMesh_0`) 0 null "None"))
  (set `self.MID` _returnvalue)
  (`MaterialInstanceDynamic.SetScalarParameterValue` (`self.MID`) "FadeParam" 0.0))

(event `OnChunkDone_Event2`
  (`MaterialInstanceDynamic.SetScalarParameterValue` (`self.MID`) "FadeParam" (/ (`KismetMathLibrary.Conv_IntToDouble` (`self.WorkDone`)) (`KismetMathLibrary.Conv_IntToDouble` (`self.WorkAmount`)))))

(fn `UserConstructionScript`
  (`parent.UserConstructionScript`))