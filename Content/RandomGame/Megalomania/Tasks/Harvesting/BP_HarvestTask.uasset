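; Harvest task actor that gathers resources from a harvestable actor for the player in Megalomania.
; It attaches to the resource, requires BPI_Harvesting, and destroys itself if that is missing or it has no workers.
; Each OnChunkDone event from the inherited timed-task logic harvests HarvestSpeed worth and passes the result to PlayerState.
; When the resource is depleted, it signals work complete and destroys itself.
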(event `self.ReceiveBeginPlay`
  (`parent.ReceiveBeginPlay`)
  (if (== (`self.Workers`) 0)
    (`self.K2_DestroyActor`)))

(event `AttachToResource`
  (params (ParentActor :type "Actor Object Reference"))
  (`self.K2_AttachToActor` ParentActor "None" "KeepRelative" "KeepRelative" "KeepRelative")
  (set `self.ResourceActor` (`self.GetAttachParentActor`))
  (if (`KismetSystemLibrary.DoesImplementInterface` (`self.ResourceActor`) "/Game/RandomGame/Megalomania/Tasks/Harvesting/BPI_Harvesting.BPI_Harvesting_C")
    (add `self.OnChunkDone` (delegate `OnChunkDone_Event_0`))
    (else
      (`self.K2_DestroyActor`))))

(event `OnChunkDone_Event_0`
  (bind (_output _bisdepleted) (message `/Game/RandomGame/Megalomania/Tasks/Harvesting/BPI_Harvesting.Harvest` (`self.ResourceActor`) (`self.HarvestSpeed`) null null))
  (`/Game/RandomGame/Megalomania/BP_MegalomaniaPS.UpdateResources` (`self.PlayerState`) _output)
  (if _bisdepleted
    (`self.OnWorkComplete`)
    (`self.K2_DestroyActor`)))

(event `self.SetupTimer`
  (if (== (`self.Workers`) 0)
    (`self.K2_DestroyActor`)
    (else
      (`parent.SetupTimer`))))

(fn `UserConstructionScript`
  (`parent.UserConstructionScript`))