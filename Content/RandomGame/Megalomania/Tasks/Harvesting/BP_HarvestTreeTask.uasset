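; Worker-driven task for harvesting a tree resource in Megalomania, built on a parent timed-task class and destroyed if it has no workers.
; It attaches to a BPI_Harvesting actor, and each completed chunk calls HarvestMessage on it, using player controller 0, to update PlayerState resources.
; The task ends when work completes or the resource is destroyed.
; An info widget is created only for the locally controlled owning player.
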(event `self.ReceiveBeginPlay`
  (`parent.ReceiveBeginPlay`)
  (if (== (`self.Workers`) 0)
    (`self.K2_DestroyActor`)
    (else
      (`self.InitInfoWidget`))))

(event `self.SetupTimer`
  (if (== (`self.Workers`) 0)
    (`self.K2_DestroyActor`)
    (else
      (`parent.SetupTimer`))))

(event `AttachToResource`
  (params (ParentActor :type "Actor Object Reference"))
  (`self.K2_AttachToActor` ParentActor "None" "KeepRelative" "KeepRelative" "KeepRelative")
  (set `self.ResourceActor` (`self.GetAttachParentActor`))
  (if (`KismetSystemLibrary.DoesImplementInterface` (`self.ResourceActor`) "/Game/RandomGame/Megalomania/Tasks/Harvesting/BPI_Harvesting.BPI_Harvesting_C")
    (add `self.OnChunkDone` (delegate `OnChunkDone_Event_0`))
    (add `self.OnDestroyed` (`self.ResourceActor`) (delegate `OnDestroyed_Event_0`))
    (add `self.OnWorkComplete` (delegate `OnWorkComplete_Event_0`))
    (else
      (`self.K2_DestroyActor`))))

(event `OnChunkDone_Event_0`
  (bind _output (message `/Game/RandomGame/Megalomania/Tasks/Harvesting/BPI_Harvesting.Harvest` (`self.ResourceActor`) (`self.HarvestSpeed`) (cast `/Game/RandomGame/Megalomania/BP_MegalomaniaPC` (`GameplayStatics.GetPlayerController` 0) :!pure true) self))
  (`/Game/RandomGame/Megalomania/BP_MegalomaniaPS.UpdateResources` (`self.PlayerState`) _output))

(event `OnDestroyed_Event_0` :!signature `self.OnDestroyed`
  (params (DestroyedActor :type "Actor Object Reference"))
  (`self.K2_DestroyActor`))

(event `OnWorkComplete_Event_0`
  (`self.K2_DestroyActor`))

(fn `InitInfoWidget`
  (bind _asbp_megalomania_pc (cast `/Game/RandomGame/Megalomania/BP_MegalomaniaPC` (`self.GetOwner`)))
  (if (`Controller.IsLocalPlayerController` _asbp_megalomania_pc)
    (bind _returnvalue (`|CreateWidget` "/Game/RandomGame/Megalomania/UI/InGame/WB_HarvestTaskInfo.WB_HarvestTaskInfo_C" _asbp_megalomania_pc self))
    (`WidgetComponent.SetWidget` (`self.TaskInfoWidget`) _returnvalue)))

(fn `UserConstructionScript`
  (`parent.UserConstructionScript`))