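; BP_BuildingGhost is a placement preview actor that shows whether a building location is valid.
; On BeginPlay it applies one dynamic instance of MM_BuildingGhost to every mesh material slot.
; Overlap events and an externally set on-landscape flag each refresh the material's IsValid scalar.
; A location is valid only when the ghost overlaps no actors and is on landscape.
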(event `self.ReceiveBeginPlay`
  (bind _returnvalue (`KismetMaterialLibrary.CreateDynamicMaterialInstance` "/Game/RandomGame/Megalomania/Tasks/Placement/MM_BuildingGhost.MM_BuildingGhost"))
  (set `self.MID` _returnvalue)
  (for _index (range (`PrimitiveComponent.GetNumMaterials` (`self.StaticMesh`)))
    (`PrimitiveComponent.SetMaterial` (`self.StaticMesh`) _index (`self.MID`))))

(event `self.ReceiveActorBeginOverlap`
  (params (OtherActor :type "Actor Object Reference"))
  (set `self.IsOverlapping?` true)
  (`self.UpdateMaterial`))

(event `self.ReceiveActorEndOverlap`
  (params (OtherActor :type "Actor Object Reference"))
  (set `self.IsOverlapping?` (> (`KismetArrayLibrary.Array_Length` (`PrimitiveComponent.GetOverlappingActors` (`self.StaticMesh`) null)) 0))
  (`self.UpdateMaterial`))

(fn `GetIsValidLocation`
  (returns (IsValidLocation :type Boolean))
  (return (and (not (`self.IsOverlapping?`)) (`self.IsOnLandscape?`))))

(fn `SetIsOnLandscape`
  (params (`IsOnLandscape?` :type Boolean))
  (set `self.IsOnLandscape?` `IsOnLandscape?`)
  (`self.UpdateMaterial`))

(fn `UpdateMaterial`
  (`MaterialInstanceDynamic.SetScalarParameterValue` (`self.MID`) "IsValid" (select `bool` (`self.GetIsValidLocation`) :`true` 1.0 :!type "Float (single-precision)")))

(fn `UserConstructionScript`)