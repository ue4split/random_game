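; Game mode for the PerfectBlend arena that handles team-based player respawning and session cleanup on logout.
; On BeginPlay, the authority caches PlayerStarts tagged RED and GREEN.
; RespawnPlayer replaces a valid pawn with a possessed TopDownCharacter, placed through RandomSpawn using the PlayerState's team, whose graph selects random team starts, with red for no team.
; Logout passes the exiting arena controller to the game instance's DestroySessionCaller.
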(event `self.ReceiveBeginPlay`
  (`/Engine/EditorBlueprintResources/ActorMacros.Switch Has Authority`
    (:`Authority`
      (bind _outactors (`GameplayStatics.GetAllActorsOfClassWithTag` "/Script/Engine.PlayerStart" "RED"))
      (set `self.SpawnPointsRED` _outactors)
      (bind _outactors_2 (`GameplayStatics.GetAllActorsOfClassWithTag` "/Script/Engine.PlayerStart" "GREEN"))
      (set `self.SpawnPointsGREEN` _outactors_2))))

(event `RespawnPlayer`
  (params (PlayerController :type "Controller Object Reference"))
  (bind _returnvalue (`Controller.K2_GetPawn` PlayerController))
  (`/Engine/EditorBlueprintResources/StandardMacros.IsValid` _returnvalue
    (:`Is Valid`
      (`self.K2_DestroyActor` _returnvalue)
      (bind _returnvalue_2 (`|SpawnActorFromClass` "/Game/TopDownBP/Blueprints/TopDownCharacter.TopDownCharacter_C" (`self.RandomSpawn` (`/Game/RandomGame/PerfectBlend/Blueprints/BP_PerfectBlendPS.Team` (cast `/Game/RandomGame/PerfectBlend/Blueprints/BP_PerfectBlendPS` (`Controller.PlayerState` PlayerController) :!pure true))) "Undefined" "OverrideRootScale" PlayerController null))
      (`Controller.Possess` PlayerController _returnvalue_2))))

(event `self.K2_OnSwapPlayerControllers`
  (params (OldPC :type "PlayerController Object Reference") (NewPC :type "PlayerController Object Reference")))

(event `self.K2_OnLogout`
  (params (ExitingController :type "Controller Object Reference"))
  (bind _asbp_perfect_blend_arena_pc (cast `/Game/RandomGame/PerfectBlend/Blueprints/BP_PerfectBlendArenaPC` ExitingController))
  (`/Game/RandomGame/Global/Blueprints/BP_RandomGameInstance.DestroySessionCaller` (cast `/Game/RandomGame/Global/Blueprints/BP_RandomGameInstance` (`GameplayStatics.GetGameInstance`) :!pure true) _asbp_perfect_blend_arena_pc))

(fn `UserConstructionScript`)