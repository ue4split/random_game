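; Lobby game mode for PerfectBlend that holds the map selection and launches the match.
; On BeginPlay it reads the first row of the map info data table and saves it as the default SelectedMap on BP_PerfectBlendGS, the game state.
; SaveMapSettings writes the chosen map info to that game state, and StartTheGame moves the session to a named map through a servertravel console command.
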(event `StartTheGame`
  (params (MapName :type String :default "/Game/RandomGame/PerfectBlend/Maps/Livada/DefaultBlendArena"))
  (`KismetSystemLibrary.ExecuteConsoleCommand` (`KismetStringLibrary.Concat_StrStr` "servertravel " MapName) null))

(event `SaveMapSettings`
  (params (MapInfo :type "/Game/RandomGame/PerfectBlend/Data/Structure/PerfectBlendMapInfo_Struct Structure"))
  (set `/Game/RandomGame/PerfectBlend/Blueprints/BP_PerfectBlendGS.SelectedMap` MapInfo (cast `/Game/RandomGame/PerfectBlend/Blueprints/BP_PerfectBlendGS` (`GameplayStatics.GetGameState`) :!pure true)))

(event `self.ReceiveBeginPlay`
  (bind _outrownames (`DataTableFunctionLibrary.GetDataTableRowNames` (`self.MapInfosDataTable`)))
  (bind _returnvalue (`|GetDataTableRow` (`self.MapInfosDataTable`) (`|GetArrayItem` _outrownames))
    (:`then`
      (`self.SaveMapSettings` _returnvalue))))

(fn `UserConstructionScript`)