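; Player controller for the Perfect Blend lobby that opens the lobby menu and syncs player identity into the player state.
; On BeginPlay it switches to UI-only input with a cursor, copies the saved player name from the game instance's user-info save into BP_PerfectBlendPS, then creates WB_LobbyMenu.
; A ChangeTeam event writes the chosen team to the same player state.
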(event `self.ReceiveBeginPlay`
  ;[1 1 1] Store Game Instance reference
  (set `self.RandomGameGI` (cast `/Game/RandomGame/Global/Blueprints/BP_RandomGameInstance` (`GameplayStatics.GetGameInstance`) :!pure true))
  ;[1 1 1] Set user input mode to UI only
  (`WidgetBlueprintLibrary.SetInputMode_UIOnlyEx` self null)
  (set `self.bShowMouseCursor` true)
  (`|ExecutionSequence`
    (:`then_0`
      (`self.RefreshPlayerState` (`/Game/RandomGame/Global/Blueprints/UserPlayerSaveGame.UserInfo` (`/Game/RandomGame/Global/Blueprints/BP_RandomGameInstance.UserInfoSaveGame` (`self.RandomGameGI`)))))
    (:`then_1`
      (`self.OpenLobbyMenu`))))

(event `OpenLobbyMenu`
  (bind _returnvalue (`|CreateWidget` "/Game/RandomGame/PerfectBlend/UI/LobbyUI/WB_LobbyMenu.WB_LobbyMenu_C" (`GameplayStatics.GetPlayerController` 0)))
  (bind _output_get (set `self.LobbyMenuWidget` _returnvalue))
  (`UserWidget.AddToViewport` _output_get 0))

(event `ChangeTeam`
  (params (Team :type "/Game/RandomGame/PerfectBlend/Blueprints/DataStructures/TeamsEnum Enum" :default "NewEnumerator0"))
  (set `/Game/RandomGame/PerfectBlend/Blueprints/BP_PerfectBlendPS.Team` Team (cast `/Game/RandomGame/PerfectBlend/Blueprints/BP_PerfectBlendPS` (`self.PlayerState`) :!pure true)))

(event `RefreshPlayerState`
  (params (UserPlayerInfo :type "/Game/RandomGame/Global/Blueprints/UserPlayerInfoStruct Structure (by ref)"))
  (set `/Game/RandomGame/PerfectBlend/Blueprints/BP_PerfectBlendPS.UserName` (`.PlayerName_9_895654F14300EA5273A5F2951AD5BEBE` (break `/Game/RandomGame/Global/Blueprints/UserPlayerInfoStruct` UserPlayerInfo)) (cast `/Game/RandomGame/PerfectBlend/Blueprints/BP_PerfectBlendPS` (`self.PlayerState`) :!pure true)))

(fn `UserConstructionScript`)