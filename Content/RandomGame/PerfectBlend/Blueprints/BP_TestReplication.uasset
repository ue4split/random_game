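; BP_TestReplication is a replication test actor that picks a random direction with zero Z on BeginPlay and stores it in Direction.
; A timeline is set up to offset its static mesh along that direction, but nothing triggers it.
; The Direction RepNotify handler is empty, and an IsServer macro branching server from client goes unused, so BeginPlay sets the direction without an authority check.
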(event `self.ReceiveBeginPlay`
  (`self.SetDirection`))

(event `SetDirection`
  (set `self.Direction` (* (`KismetMathLibrary.Normal` (`KismetMathLibrary.RandomUnitVector`)) (1.0 1.0 0.0))))

(fn `OnRep_Direction`)

(fn `UserConstructionScript`)