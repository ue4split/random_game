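; Spawn volume actor that periodically spawns Vegemon pawns at random points inside its box component.
; A looping timer rolls a spawn chance that falls linearly as the world count of that class approaches the maximum, acting as soft population control.
; Each spawned pawn gets its default controller, and a BP_VegetableController receives a reference back to this volume.
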(event `self.ReceiveBeginPlay`
  (bind _returnvalue (`KismetSystemLibrary.K2_SetTimerDelegate` (delegate `SpawnVegemon`) (`self.SpawnInterval`) true))
  (set `self.Timer` _returnvalue))

(event `SpawnVegemon`
  (bind (_origin _boxextent) (`KismetSystemLibrary.GetComponentBounds` (`self.SpawnBox`)))
  ;[1 1 1] Population control (Max World Count)
  (bind _outactors (`GameplayStatics.GetAllActorsOfClass` (`self.VegemonClass`)))
  (if (>= (- 1.0 (/ (`KismetMathLibrary.Conv_IntToDouble` (`KismetArrayLibrary.Array_Length` _outactors)) (`self.MaxWorldCount`))) (`KismetMathLibrary.RandomFloat`))
    ;[1 1 1] Spawn the vegemon
    (bind _returnvalue (`|SpawnActorFromClass` (`self.VegemonClass`) (`KismetMathLibrary.MakeTransform` (`KismetMathLibrary.RandomPointInBoundingBox` _origin _boxextent)) "AdjustIfPossibleButAlwaysSpawn" "OverrideRootScale" null null))
    (`Pawn.SpawnDefaultController` _returnvalue)
    (bind _asbp_vegetable_controller (cast `/Game/RandomGame/PerfectBlend/Vegetables/Blueprints/BP_VegetableController` (`Pawn.GetController` _returnvalue)))
    (set `/Game/RandomGame/PerfectBlend/Vegetables/Blueprints/BP_VegetableController.SpawnVolumeReference` self _asbp_vegetable_controller)))

(fn `UserConstructionScript`)