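; BP_VegetableController is the AI controller for vegetable pawns that can be caught, escape or be blended, running the BT_Broccoli behavior tree from BeginPlay.
; OnCaught stops the brain logic and messages the pawn to attach to the player's carry socket.
; OnEscape frees the pawn from the grab and restarts the logic.
; OnBlend frees it, then destroys pawn and controller after a short delay, with the blend animation still TODO.
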(event `self.ReceiveBeginPlay`
  (`self.RunBehaviorTree` "/Game/RandomGame/PerfectBlend/Vegetables/Livada/Broccoli/BT_Broccoli.BT_Broccoli"))

(event `OnCaught`
  (params (PlayerCharacter :type "/Game/RandomGame/PerfectBlend/Characters/PerfectBlendCharacter Object Reference"))
  (`BrainComponent.StopLogic` (`self.BrainComponent`) "")
  (message `/Game/RandomGame/PerfectBlend/Vegetables/Blueprints/BI_Vegetable.AttachToCarrySocket` (`self.K2_GetPawn`) PlayerCharacter))

(event `OnEscape`
  (message `/Game/RandomGame/PerfectBlend/Vegetables/Blueprints/BI_Vegetable.FreeFromPlayerGrab` (`self.K2_GetPawn`))
  (`BrainComponent.RestartLogic` (`self.BrainComponent`)))

(event `OnBlend`
  (message `/Game/RandomGame/PerfectBlend/Vegetables/Blueprints/BI_Vegetable.FreeFromPlayerGrab` (`self.K2_GetPawn`))
  ;[1 1 1] TODO blend animation
  (`KismetSystemLibrary.Delay` 0.6)
  (`self.K2_DestroyActor` (`self.K2_GetPawn`))
  (`self.K2_DestroyActor`))

(fn `UserConstructionScript`)