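; Cauliflower vegetable character that the player can carry and that can be blended.
; On grab, it disables movement and collision and snaps to the player mesh's carry socket; on release, it detaches, restores collision and starts falling.
; The blend-and-destroy event defers to its parent implementation.
; Its default behavior tree is BT_Broccoli, the broccoli's tree, rather than a cauliflower-specific one.
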(event `self.AttachToCarrySocket`
  (params (PlayerCharacter :type "/Game/RandomGame/PerfectBlend/Characters/PerfectBlendCharacter Object Reference"))
  ;[1 1 1] Disable movement component
  (`CharacterMovementComponent.DisableMovement` (`self.CharacterMovement`))
  ;[1 1 1] Disable collisions
  (`PrimitiveComponent.SetCollisionEnabled` (`self.Mesh`) "NoCollision")
  (`PrimitiveComponent.SetCollisionEnabled` (`self.CapsuleComponent`) "NoCollision")
  ;[1 1 1] Attach to Carry socket on player character
  (`self.K2_AttachToComponent` (`Character.Mesh` PlayerCharacter) "CarryVegetableSocket" "SnapToTarget" "SnapToTarget" "SnapToTarget"))

(event `self.FreeFromPlayerGrab`
  (`self.K2_DetachFromActor` "KeepWorld" "KeepRelative" "KeepWorld")
  (`PrimitiveComponent.SetCollisionEnabled` (`self.Mesh`) "QueryAndPhysics")
  (`PrimitiveComponent.SetCollisionEnabled` (`self.CapsuleComponent`) "QueryAndPhysics")
  (`CharacterMovementComponent.SetMovementMode` (`self.CharacterMovement`) "MOVE_Falling" 0))

(event `self.DoBlendAndDestroy`
  (`parent.DoBlendAndDestroy`))

(fn `GetDefaultBehaviorTree`
  (returns (BehaviorTree :type "BehaviorTree Object Reference"))
  (return "/Game/RandomGame/PerfectBlend/Vegetables/Livada/Broccoli/AI/BT_Broccoli.BT_Broccoli"))

(fn `UserConstructionScript`)